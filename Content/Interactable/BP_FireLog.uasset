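; BP_FireLog is an interactable log that stokes the fire by adding its refill time to the BP_Fire actor found at BeginPlay.
; Interaction and hover highlight work only once the fire's remaining time drops to half its dimming start time or lower.
; The highlight toggles custom depth rendering on the static mesh components.
; It reports a fixed interaction type and flags itself as single.
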(event `self.ReceiveBeginPlay`
  (bind _returnvalue (`GameplayStatics.GetActorOfClass` "/Game/Interactable/Fire/BP_Fire.BP_Fire_C"))
  (set `self.FireLight` _returnvalue))

(event `/Game/Interactable/I_Interactable.InteractBegin`
  (bind _firelight (`self.FireLight`))
  ;[1 1 1] Start Interaction
  (if (`self.IsLightDimingPercent` 0.5)
    (`/Game/Interactable/Fire/BP_Fire.AddTime` _firelight (`/Game/Interactable/Fire/BP_Fire.Refill` _firelight))
    (`KismetSystemLibrary.PrintString` "Stoke The Fire")))

(event `/Game/Interactable/I_Interactable.onHoverEnter`
  ;[1 1 1] Toggles interactable border
  (if (`self.IsLightDimingPercent` 0.5)
    (`PrimitiveComponent.SetRenderCustomDepth` (`self.K2_GetComponentsByClass` "/Script/Engine.StaticMeshComponent") true)))

(event `/Game/Interactable/I_Interactable.onHoverExit`
  ;[1 1 1] Toggles interactable border
  (`PrimitiveComponent.SetRenderCustomDepth` (`self.K2_GetComponentsByClass` "/Script/Engine.StaticMeshComponent") false))

(fn `GetType`
  (returns (InteractableType :type "/Game/Interactable/E_InteractableTypes Enum"))
  (return "NewEnumerator0"))

(fn `IsLightDiming`
  (returns (ReturnValue :type Boolean))
  (bind _firelight (`self.FireLight`))
  (return (<= (`/Game/Interactable/Fire/BP_Fire.TimeLeft` _firelight) (`/Game/Interactable/Fire/BP_Fire.StartDimTime` _firelight))))

(fn `IsLightDimingPercent`
  (params (percent :type "Float (double-precision)"))
  (returns (ReturnValue :type Boolean))
  (bind _firelight (`self.FireLight`))
  (return (<= (/ (`/Game/Interactable/Fire/BP_Fire.TimeLeft` _firelight) (`KismetMathLibrary.Conv_IntToDouble` (`/Game/Interactable/Fire/BP_Fire.StartDimTime` _firelight))) percent)))

(fn `isSingle`
  (returns (isSingle :type Boolean))
  (return true))

(fn `UserConstructionScript`)