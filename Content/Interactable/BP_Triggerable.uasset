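; BP_Triggerable is an interactable puzzle object that triggers once the player enters a key sequence (Password).
; Hovering toggles custom depth on its static meshes as a highlight, and the first interaction adds its Quest through the game mode.
; OnPasswordKey checks each key by index, counts matches and, after the last one, either sets completion state and calls Trigger, or flags failure.
; ResetPasswordIndex clears the counters and failure flag.
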(event `/Game/Interactable/I_Interactable.onHoverEnter`
  ;[1 1 1] Toggles interactable border
  (`PrimitiveComponent.SetRenderCustomDepth` (`self.K2_GetComponentsByClass` "/Script/Engine.StaticMeshComponent") true))

(event `OnComplete`
  ;[1 0.9843 0.5333] Completed
)

(event `/Game/Interactable/I_Interactable.onHoverExit`
  ;[1 1 1] Toggles interactable border
  (`PrimitiveComponent.SetRenderCustomDepth` (`self.K2_GetComponentsByClass` "/Script/Engine.StaticMeshComponent") false))

(event `OnCorrectKey`
  ;[0.5117 1 0.5418] Correct Key
)

(event `OnSuccess`
  ;[0.5433 1 0.6575] Successfully completed puzzle
  (set `self.state` "NewEnumerator2")
  (set `self.isComplete` true)
  (`self.Trigger`))

(event `/Game/Interactable/I_Interactable.InteractBegin`
  ;[1 1 1] handle quest creation
  (`/Engine/EditorBlueprintResources/StandardMacros.DoOnce` false
    (:`Completed`
      (`/Game/ThirdPerson/Blueprints/BP_ThirdPersonGameMode.AddQuest` (cast `/Game/ThirdPerson/Blueprints/BP_ThirdPersonGameMode` (`GameplayStatics.GetGameMode`) :!pure true) (`self.Quest`))
      (set `self.state` "NewEnumerator1"))))

(event `OnWrongKey`
  (params (key :type Name))
  ;[1 0.5581 0.6179] Wrong Key
  (`KismetSystemLibrary.PrintString` (`KismetStringLibrary.Concat_StrStr` "Got: " (`KismetStringLibrary.Conv_NameToString` key) " Expected: " (`KismetStringLibrary.Conv_IntToString` (`KismetArrayLibrary.Array_Length` (`self.Password`))))))

(event `OnFailure`
  ;[1 0.5507 0.5308] Failed to complete puzzle
  (set `self.isFailed` true)
  (`KismetSystemLibrary.PrintString` (`KismetStringLibrary.Concat_StrStr` "Failed: " (`KismetStringLibrary.Conv_NameToString` (`self.Quest`)))))

(event `/Game/Interactable/I_Password.ResetPasswordIndex`
  ;[1 1 1] Reset Password Index
  (set `self.NumCorrect` 0)
  (set `self.index` 0)
  (set `self.isFailed` false))

(fn `CheckPassword`
  (params (key :type Name) (index :type Integer))
  (returns (isValid :type Boolean))
  (locals (NewLocalVar :type Name :default "None"))
  (bind _returnvalue (== (`|GetArrayItem` (`self.Password`) index) key))
  (if (`KismetArrayLibrary.Array_IsValidIndex` (`self.Password`) index)
    (if _returnvalue
      (`self.OnCorrectKey`)
      (else
        (`self.OnWrongKey` key)))
    (return _returnvalue)
    (else
      (return false))))

(fn `isSingle`
  (returns (isSingle :type Boolean))
  (return true))

(fn `onPasswordKey`
  (params (key :type Name))
  (returns (isCorrect :type Boolean) (isDone :type Boolean))
  (locals (isValid :type Boolean :default false) (isComplete :type Boolean))
  (if (`self.isComplete`)
    (return false true)
    (else
      (bind _isvalid (`/Game/Interactable/I_Password.CheckPassword` key (`self.index`)))
      (bind _output_get (set `local.isValid` _isvalid))
      (if _output_get
        (`/Engine/EditorBlueprintResources/StandardMacros.IncrementInt` (`self.NumCorrect`)
          (:`  `
            _)))
      (`/Engine/EditorBlueprintResources/StandardMacros.IncrementInt` (`self.index`)
        (:`  `
          (bind _output_get_2 (set `local.isComplete` (>= (`self.index`) (`KismetArrayLibrary.Array_Length` (`self.Password`)))))
          (if _output_get_2
            (`self.OnComplete`)
            (if (>= (`self.NumCorrect`) (`KismetArrayLibrary.Array_Length` (`self.Password`)))
              (`self.OnSuccess`)
              (else
                (`self.OnFailure`)))
            (return (`local.isValid`) true)
            (else
              (return (`local.isValid`) false))))))))

(fn `UserConstructionScript`
  (`parent.UserConstructionScript`))