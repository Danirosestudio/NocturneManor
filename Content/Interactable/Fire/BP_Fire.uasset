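; Interactable fire that acts as a countdown, printing "Game over" once its time and bonus grace period run out.
; A looping one-second timer decrements and logs the time left, updating point light intensity and switching the LightFlicker material collection parameter off below zero.
; Interacting calls AddTime with the refill amount to top up the timer.
; Hovering toggles custom depth on static meshes for an interactable outline.
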(event `/Game/Interactable/I_Interactable.onHoverEnter`
  ;[1 1 1] Toggles interactable border
  (`PrimitiveComponent.SetRenderCustomDepth` (`self.K2_GetComponentsByClass` "/Script/Engine.StaticMeshComponent") true))

(event `/Game/Interactable/I_Interactable.onHoverExit`
  ;[1 1 1] Toggles interactable border
  (`PrimitiveComponent.SetRenderCustomDepth` (`self.K2_GetComponentsByClass` "/Script/Engine.StaticMeshComponent") false))

(event `self.ReceiveBeginPlay`
  ;[1 1 1] Setup
  (`KismetSystemLibrary.K2_SetTimer` null "OnTimeTIcks" 1.0 true)
  (set `self.TimeLeft` (`self.Time`))
  (`/Engine/EditorBlueprintResources/StandardMacros.NegateInt` (`self.Bonus Time`)
    (:`  `
      (set `self.IntensityMax` (`LightComponentBase.Intensity` (`self.PointLight`))))))

(event `OnTimeTIcks`
  (bind _intensitymax (`self.IntensityMax`))
  (bind _intensitymin (`self.IntensityMin`))
  ;[1 1 1] Timer call back function
  (if (>= (`self.TimeLeft`) (`self.Bonus Time`))
    (bind _result (`/Engine/EditorBlueprintResources/StandardMacros.DecrementInt` (`self.TimeLeft`))
      (:`  `
        (`KismetSystemLibrary.PrintString` (`KismetStringLibrary.Conv_IntToString` _result))
        ;;[1 0.6547 0.6348] Over Time
        (if (< _result 0)
          (`KismetMaterialLibrary.SetScalarParameterValue` "/Game/Interactable/Fire/MP_Light.MP_Light" "LightFlicker")
          (if (== (`self.TimeLeft`) (`self.Bonus Time`))
            (`self.OnEnd`))
          (else
            ;;[1 0.9613 0.5059] Change Intensity
            (`LightComponent.SetIntensity` (`self.PointLight`) (`KismetMathLibrary.FClamp` (`KismetMathLibrary.Lerp` _intensitymin _intensitymax (/ (`KismetMathLibrary.Max` (`self.TimeLeft`)) (`KismetMathLibrary.Conv_IntToDouble` (`self.StartDimTime`)))) _intensitymin _intensitymax))
            (`KismetMaterialLibrary.SetScalarParameterValue` "/Game/Interactable/Fire/MP_Light.MP_Light" "LightFlicker" 1.0)))))))

(event `/Game/Interactable/I_Interactable.InteractBegin`
  ;[1 1 1] Interact Event Refill
  (`self.AddTime` (`self.Refill`)))

(event `OnEnd`
  ;[1 1 1] Handle End Logic
  (`KismetSystemLibrary.PrintString` "Game over"))

(fn `AddTime`
  (params (Time :type Integer))
  (set `self.TimeLeft` (`KismetMathLibrary.Min` (+ Time (`self.TimeLeft`)) (`self.Time`)))
  (return))

(fn `isSingle`
  (returns (isSingle :type Boolean))
  (return true))

(fn `UserConstructionScript`)