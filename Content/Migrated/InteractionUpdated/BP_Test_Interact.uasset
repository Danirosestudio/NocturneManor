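; BP_Test_Interact is a test interactable actor that visibly responds when interacted with.
; InteractEvent drives a FlipFlop that alternates the first material slot of HighlightedMesh between two basic materials.
; The construction script runs the parent's script, then sets TextRender to the actor's display name as a label.
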(event `self.InteractEvent`
  (params (Player :type "/Game/ThirdPerson/Blueprints/BP_ThirdPersonCharacter Object Reference"))
  (`/Engine/EditorBlueprintResources/StandardMacros.FlipFlop`
    (:`A`
      (`PrimitiveComponent.SetMaterial` (`self.HighlightedMesh`) 0 "/Engine/MapTemplates/Materials/BasicAsset01.BasicAsset01"))
    (:`B`
      (`PrimitiveComponent.SetMaterial` (`self.HighlightedMesh`) 0 "/Engine/MapTemplates/Materials/BasicAsset02.BasicAsset02"))))

(fn `UserConstructionScript`
  (`parent.UserConstructionScript`)
  (`TextRenderComponent.K2_SetText` (`self.TextRender`) (`KismetTextLibrary.Conv_StringToText` (`KismetSystemLibrary.GetDisplayName` self))))