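; Base interactable Blueprint that responds to hover and player interaction, with an empty InteractEvent hook for children.
; The construction script gathers its static mesh components, and AddMesh can extend that list for custom-depth highlighting.
; Hover and interact fire event dispatchers, with hover-enter and interact gated by Interactable.
; Single-use objects disable interaction and clear the highlight before InteractEvent runs.
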(event `self.ReceiveBeginPlay`)

(event `/Game/Migrated/InteractionUpdated/I_Interact.Interact`
  (params (Player :type "/Game/ThirdPerson/Blueprints/BP_ThirdPersonCharacter Object Reference"))
  ;[1 1 1] Interact
  (if (`self.Interactable`)
    (if (`self.Single`)
      (`self.DisableInteract`))
    (`self.InteractEvent` Player)
    (`self.OnInteract` Player)))

(event `/Game/Migrated/InteractionUpdated/I_Hover.HoverEnter`
  ;[1 1 1] Hover
  (if (`self.Interactable`)
    (`self.ToggleHighlight` (`self.HighlightEnabled`))
    (`self.OnHoverEnter`)))

(event `/Game/Migrated/InteractionUpdated/I_Hover.HoverExit`
  ;[1 1 1] Hover
  (`self.ToggleHighlight` false)
  (`self.OnHoverExit`))

(event `InteractEvent`
  (params (Player :type "/Game/ThirdPerson/Blueprints/BP_ThirdPersonCharacter Object Reference")))

(fn `AddMesh`
  (params (Mesh :type "StaticMeshComponent Object Reference (by ref)"))
  (`KismetArrayLibrary.Array_Add` (`self.StaticMeshList`) Mesh)
  (return))

(fn `DisableInteract`
  (bind _output_get (set `self.Interactable` false))
  (`self.ToggleHighlight` _output_get))

(fn `ToggleHighlight`
  (params (bValue :type Boolean))
  (`PrimitiveComponent.SetRenderCustomDepth` (`self.StaticMeshList`) bValue)
  (return))

(fn `UserConstructionScript`
  (set `self.StaticMeshList` (`self.K2_GetComponentsByClass` "/Script/Engine.StaticMeshComponent")))