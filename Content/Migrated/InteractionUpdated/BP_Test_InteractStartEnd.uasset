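; BP_Test_InteractStartEnd is a test actor for the interaction system's begin and end events.
; BeginInteract switches the first material slot of StaticMeshList to BasicAsset01, and EndInteract switches it to BasicShapeMaterial.
; The construction script calls its parent, then sets TextRender to the actor's display name as a label.
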(event `/Game/Migrated/InteractionUpdated/I_InteractStartEnd.BeginInteract`
  (params (Player :type "/Game/ThirdPerson/Blueprints/BP_ThirdPersonCharacter Object Reference"))
  (`PrimitiveComponent.SetMaterial` (`self.StaticMeshList`) 0 "/Engine/MapTemplates/Materials/BasicAsset01.BasicAsset01"))

(event `/Game/Migrated/InteractionUpdated/I_InteractStartEnd.EndInteract`
  (params (Player :type "/Game/ThirdPerson/Blueprints/BP_ThirdPersonCharacter Object Reference"))
  (`PrimitiveComponent.SetMaterial` (`self.StaticMeshList`) 0 "/Engine/BasicShapes/BasicShapeMaterial.BasicShapeMaterial"))

(fn `UserConstructionScript`
  (`parent.UserConstructionScript`)
  (`TextRenderComponent.K2_SetText` (`self.TextRender`) (`KismetTextLibrary.Conv_StringToText` (`KismetSystemLibrary.GetDisplayName` self))))