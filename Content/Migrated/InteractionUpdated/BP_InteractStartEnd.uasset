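; Interactable Blueprint for interactions with a start and an end, during which the object takes over control from the player.
; Beginning hands input to itself, hides the player, sets Game-and-UI input mode, applies cursor and highlight settings, then calls begin hooks.
; Its own IA_Interact input calls ResumeGame to reverse this without a player line trace, restoring game-only input and calling end hooks.
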(event `self.ReceiveBeginPlay`
  (add `self.OnInteract` (`|CreateDelegate` :!event `Begin`)))

(event `EnhancedInput|/Game/ThirdPerson/Input/Actions/IA_Interact`
  (params (ActionValue :type Boolean) (ElapsedSeconds :type "Float (double-precision)") (TriggeredSeconds :type "Float (double-precision)") (InputAction :type "InputAction Object Reference" :default "/Game/ThirdPerson/Input/Actions/IA_Interact.IA_Interact"))
  ;[1 1 1] Handle End Event w/o using player line trace
  (:`Started`
    (`self.ResumeGame`)))

(fn `Begin`
  (params (Player :type "/Game/ThirdPerson/Blueprints/BP_ThirdPersonCharacter Object Reference"))
  (bind _output_get (set `self.Player` Player))
  (`self.TransferInput` _output_get self (`self.ShowMouseDuringInteraction`))
  (set `self.IsInteracting` true)
  (`self.ToggleHighlight` (`self.ShowHighlightDuringInteraction`))
  (`WidgetBlueprintLibrary.SetInputMode_GameAndUIEx` (`GameplayStatics.GetPlayerController` 0) null "LockAlways")
  (`self.SetActorHiddenInGame` (`self.Player`) true)
  (`self.BeginInteract` (`self.Player`))
  (`self.OnInteractBegin`)
  (return))

(fn `ResumeGame`
  (`self.TransferInput` self (`self.Player`))
  (set `self.IsInteracting` false)
  (`self.ToggleHighlight` (and (`self.HighlightEnabled`) (`self.Interactable`)))
  (`WidgetBlueprintLibrary.SetInputMode_GameOnly` (`GameplayStatics.GetPlayerController` 0))
  (`self.SetActorHiddenInGame` (`self.Player`) false)
  (`self.EndInteract` (`self.Player`))
  (`self.OnInteractEnd`)
  (return))

(fn `TransferInput`
  (params (DisableTarget :type "Actor Object Reference") (EnableTarget :type "Actor Object Reference") (`Show Mouse Cursor` :type Boolean))
  (`self.DisableInput` DisableTarget (`GameplayStatics.GetPlayerController` 0))
  (`self.EnableInput` EnableTarget (`GameplayStatics.GetPlayerController` 0))
  (set `PlayerController.bShowMouseCursor` `Show Mouse Cursor` (`GameplayStatics.GetPlayerController` 0))
  (return))

(fn `UserConstructionScript`
  (`parent.UserConstructionScript`))