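; AC_CameraBlend is a component that toggles the first player's view between its owning actor and the player character with a blended camera transition.
; Each Trigger call alternates through a FlipFlop, and TransitionCamera applies the view target blend with the outgoing view locked.
; Blending to the owner starts a timer matching the blend time that fires OnComplete.
; Blending back clears that timer and fires OnExit immediately.
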(event `/Game/Migrated/InteractionUpdated/I_Trigger.Trigger`
  (`/Engine/EditorBlueprintResources/StandardMacros.FlipFlop`
    (:`A`
      (`self.TransitionCamera` (`self.GetOwner`))
      (bind _returnvalue (`KismetSystemLibrary.K2_SetTimerDelegate` (delegate `CompleteTimer`) (`self.Blend Time`)))
      (set `self.Time Handler` _returnvalue))
    (:`B`
      (`self.TransitionCamera` (`GameplayStatics.GetPlayerCharacter` 0))
      (`KismetSystemLibrary.K2_ClearAndInvalidateTimerHandle` (`self.Time Handler`))
      (`self.OnExit`))))

(event `CompleteTimer`
  (`self.OnComplete`))

(fn `TransitionCamera`
  (params (NewViewTarget :type "Actor Object Reference"))
  (`PlayerController.SetViewTargetWithBlend` (`GameplayStatics.GetPlayerController` 0) NewViewTarget (`self.Blend Time`) "VTBlend_Linear" (`self.Blend Exp`) true))