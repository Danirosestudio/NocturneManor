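; Base interactable actor that starts a camera blend when interacted with.
; Both begin and end interact events call Trigger on its AC_CameraBlend component.
; The component's completion and exit callbacks print debug messages and swap the material on HighlightedMesh, giving visible feedback for each camera state.
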(event `/Game/Migrated/InteractionUpdated/I_InteractStartEnd.BeginInteract`
  (params (Player :type "/Game/ThirdPerson/Blueprints/BP_ThirdPersonCharacter Object Reference"))
  (`/Game/Migrated/InteractionUpdated/I_Trigger.Trigger` (`self.AC_CameraBlend`)))

(event `/Game/Migrated/InteractionUpdated/I_InteractStartEnd.EndInteract`
  (params (Player :type "/Game/ThirdPerson/Blueprints/BP_ThirdPersonCharacter Object Reference"))
  (`/Game/Migrated/InteractionUpdated/I_Trigger.Trigger` (`self.AC_CameraBlend`)))

(event `self.AC_CameraBlend.OnComplete`
  (`KismetSystemLibrary.PrintString` "Camera Finished")
  (`PrimitiveComponent.SetMaterial` (`self.HighlightedMesh`) 0 "/Engine/MapTemplates/Materials/BasicAsset01.BasicAsset01"))

(event `self.AC_CameraBlend.OnExit`
  (`KismetSystemLibrary.PrintString` "Camera Exit")
  (`PrimitiveComponent.SetMaterial` (`self.HighlightedMesh`) 0 "/Engine/BasicShapes/BasicShapeMaterial.BasicShapeMaterial"))

(fn `UserConstructionScript`
  (`parent.UserConstructionScript`))