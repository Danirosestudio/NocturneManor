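; AC_MenuController is a menu controller component that forwards menu operations to a MenuDataAsset.
; On BeginPlay it binds to the data asset's OnLoad event and rebroadcasts the loaded widget through its own OnLoad dispatcher.
; Open, Close and GetWidget are thin wrappers over the data asset, which owns the widget and the actual menu logic.
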(event `self.ReceiveBeginPlay`
  (add `/Game/Migrated/DataAssets/Event/DA_Ev_Menu.OnLoad` (`self.MenuDataAsset`) (delegate `Loaded`)))

(event `Loaded`
  (params (Widget :type "Widget Object Reference"))
  (`self.OnLoad` Widget))

(fn `Close`
  (`/Game/Migrated/DataAssets/Event/DA_Ev_Menu.Close` (`self.MenuDataAsset`)))

(fn `GetWidget`
  (returns (Widget :type "Widget Object Reference"))
  (return (`/Game/Migrated/DataAssets/Event/DA_Ev_Menu.Widget` (`self.MenuDataAsset`))))

(fn `Open`
  (`/Game/Migrated/DataAssets/Event/DA_Ev_Menu.Open` (`self.MenuDataAsset`)))