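; Musical dial puzzle that blends the camera on interact, then lets the player turn dials to enter a note sequence.
; Move input rolls the current dial, stores and plays each new note at roughly 45-degree detents, and snaps on release.
; Jump rotates the mesh 120 degrees to the next dial, cycling through three.
; The last key triggers an answer check: success animates the cone open and ends interaction, failure resets the dials.
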(event `self.ReceiveBeginPlay`
  ;[1 1 1 0.5] Event Begin
  (`parent.ReceiveBeginPlay`)
  (set `self.Relative Rotation` (`SceneComponent.K2_GetComponentRotation` (`self.DefaultSceneRoot`)))
  (`TimelineComponent.SetPlayRate` (`self.ResetTimeLine`) 2.0))

(event `/Game/Migrated/InteractionUpdated/I_InteractStartEnd.BeginInteract`
  (params (Player :type "/Game/ThirdPerson/Blueprints/BP_ThirdPersonCharacter Object Reference"))
  ;[1 1 1 0.5] Interact
  (`/Game/Migrated/Camera/AC_CameraBlend.Trigger` (`self.AC_CameraBlend`)))

(event `/Game/Migrated/InteractionUpdated/I_InteractStartEnd.EndInteract`
  (params (Player :type "/Game/ThirdPerson/Blueprints/BP_ThirdPersonCharacter Object Reference"))
  ;[1 1 1 0.5] Interact
  (`/Game/Migrated/Camera/AC_CameraBlend.Trigger` (`self.AC_CameraBlend`))
  (set `self.IsActive` false))

(event `EnhancedInput|/Game/ThirdPerson/Input/Actions/IA_Move`
  (params (ActionValue :type "Vector2D Structure") (ElapsedSeconds :type "Float (double-precision)") (TriggeredSeconds :type "Float (double-precision)") (InputAction :type "InputAction Object Reference" :default "/Game/ThirdPerson/Input/Actions/IA_Move.IA_Move"))
  ;[1 1 1] Handle Rotate Dials
  (:`Triggered`
    (`self.CanInteractPuzzle`
      (:`IsValid`
        (if (!= ActionValue_X 0.0)
          (bind _dial (`self.GetDial`))
          (`SceneComponent.K2_AddRelativeRotation` _dial (`KismetMathLibrary.MakeRotator` (* ActionValue_X -1.0)) false false)
          (bind _relativerotation_roll (`KismetMathLibrary.BreakRotator` (`SceneComponent.RelativeRotation` _dial)))
          (if (`self.IsNoteAngle` _relativerotation_roll)
            (`/Engine/EditorBlueprintResources/StandardMacros.DoOnce` false :!label _label
              (:`Completed`
                (bind _value (`self.CalcValueRotation` _relativerotation_roll))
                (if (not (`self.IsSameNote` _value))
                  (`self.UpdateData` _value))))
            (else
              (goto _label :!via `Reset`)))))))
  (:`Completed`
    (`self.CanInteractPuzzle`
      (:`IsValid`
        (`self.SnapToEnd`)))))

(event `self.AC_CameraBlend.OnComplete`
  ;[1 1 1 0.5] Interact
  (set `self.IsActive` true))

(event `RotateNext`
  ;[1 1 1] Rotate NExt
  (bind (_direction _newtrack_0) (`Timeline|RotateTimeLine` :!via `PlayFromStart`)
    (:`Update`
      (`self.UpdateRotation` _newtrack_0 (`self.CurrentRotation`) (+ (`self.CurrentRotation`) 1)))
    (:`Finished`
      (`/Engine/EditorBlueprintResources/StandardMacros.IncrementInt` (`self.CurrentRotation`)
        (:`  `
          (set `self.IsActive` true))))))

(event `EnhancedInput|/Game/ThirdPerson/Input/Actions/IA_Jump`
  (params (ActionValue :type Boolean) (ElapsedSeconds :type "Float (double-precision)") (TriggeredSeconds :type "Float (double-precision)") (InputAction :type "InputAction Object Reference" :default "/Game/ThirdPerson/Input/Actions/IA_Jump.IA_Jump"))
  ;[1 1 1] Handle Next click
  (:`Started`
    (`self.CanInteractPuzzle`
      (:`IsValid`
        (if (== (`self.CurrentRotation`) (- (`KismetArrayLibrary.Array_Length` (`self.Keys`)) 1))
          (bind _iscorrect1 (`self.CheckCompleted`))
          (if _iscorrect1
            (`self.FakeOpen`)
            (`GameplayStatics.PlaySound2D` "/Engine/EditorSounds/Notifications/CompileSuccess.CompileSuccess" 1.0 1.0 0.0 null null)
            (else
              (`self.ResetRotate`)
              (`GameplayStatics.PlaySound2D` "/Engine/EditorSounds/Notifications/CompileFailed.CompileFailed" 1.0 1.0 0.0 null null)))
          (else
            (`self.RotateNext`)
            (set `self.IsActive` false)))))))

(event `ResetRotate`
  ;[1 1 1] Reset Animation
  (`SceneComponent.K2_SetRelativeRotation` :`self` (`self.Dial_1`))
  (`SceneComponent.K2_SetRelativeRotation` :`self` (`self.Dial_3`))
  (`SceneComponent.K2_SetRelativeRotation` :`self` (`self.Dail_2`))
  (bind (_direction _newtrack_0) (`Timeline|ResetTimeLine` :!via `PlayFromStart`)
    (:`Update`
      (`self.UpdateRotation` _newtrack_0 (`self.CurrentRotation`)))
    (:`Finished`
      (set `self.CurrentRotation` 0)
      (set `self.IsActive` true))))

(event `FakeOpen`
  ;[1 1 1] Open Animation
  (`PrimitiveComponent.SetMaterial` (`self.Cone`) 0 "/Engine/MapTemplates/Materials/BasicAsset03.BasicAsset03")
  (bind (_direction _newtrack_0 _newtrack_2) (`Timeline|OpenTimeLine` :!via `PlayFromStart`)
    (:`Update`
      (`SceneComponent.K2_SetRelativeTransform` (`self.Cone`) (`KismetMathLibrary.MakeTransform` (`KismetMathLibrary.MakeVector` 0.0 0.0 (`KismetMathLibrary.Lerp` 65.0 75.0 _newtrack_0)) (struct) (`KismetMathLibrary.Conv_DoubleToVector` (`KismetMathLibrary.Lerp` 0.1 0.3 _newtrack_2))) false false))
    (:`Finished`
      (`self.DisableInteract`)
      (`self.ResumeGame`))))

(fn `CheckCompleted`
  (returns (isCorrect1 :type Boolean))
  (locals (isCorrect :type Boolean :default true))
  (for (_array_element _array_index) (`self.Keys`)
    (if (not (== _array_element (`|GetArrayItem` (`self.Answer`) _array_index)))
      (set `local.isCorrect` false)
      (break)))
  (return (`local.isCorrect`)))

(fn `GetDial`
  (returns (Dial :type "StaticMeshComponent Object Reference"))
  (switch `int` (mod (`self.CurrentRotation`) 3)
    (:`0`
      (return (`self.Dial_1`)))
    (:`1`
      (return (`self.Dail_2`)))
    (:`2`
      (return (`self.Dial_3`)))))

(fn `IsNoteAngle`
  (params (Angle :type "Float (double-precision)"))
  (returns (IsValid :type Boolean))
  (return (<= (mod (+ (`KismetMathLibrary.Abs` Angle) (/ (`self.ExpandedDetectAngle`) 2)) 45.0) (`self.ExpandedDetectAngle`))))

(fn `IsSameNote`
  (params (B :type Integer))
  (returns (ReturnValue :type Boolean))
  (return (== B (`|GetArrayItem` (`self.Keys`) (`self.CurrentRotation`)))))

(fn `SnapToEnd`
  (locals (LocalDial :type "StaticMeshComponent Object Reference"))
  (bind _relativerotation_roll (`KismetMathLibrary.BreakRotator` (`SceneComponent.RelativeRotation` (`local.LocalDial`))))
  (bind (_value _rotation) (`self.CalcValueRotation` _relativerotation_roll))
  (bind _dial (`self.GetDial`))
  (set `local.LocalDial` _dial)
  (if (not (`self.IsSameNote` _value))
    (`self.UpdateData` _value))
  (`SceneComponent.K2_SetRelativeRotation` (`local.LocalDial`) (`KismetMathLibrary.MakeRotator` _rotation) false false)
  (return))

(fn `UpdateData`
  (params (Value :type "Integer (by ref)"))
  (`KismetArrayLibrary.Array_Set` (`self.Keys`) (`self.CurrentRotation`) Value)
  (bind _sound (`/Game/Migrated/DataAssets/MusicKeys/DA_MusicKeys.GetSoundByIndex` (`self.MusicNotes`) Value))
  (`GameplayStatics.PlaySound2D` _sound 1.0 1.0 0.0 null null))

(fn `UpdateRotation`
  (params (TrackProgress :type "Float (double-precision)") (Start :type Integer) (End :type Integer))
  (`SceneComponent.K2_SetWorldRotation` (`self.StaticMesh`) (`KismetMathLibrary.ComposeRotators` (`self.Relative Rotation`) (`KismetMathLibrary.MakeRotator` 0.0 0.0 (`KismetMathLibrary.Lerp` (* Start 120.0) (* End 120.0) TrackProgress))) false false))

(fn `UserConstructionScript`)