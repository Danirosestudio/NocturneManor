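; Interactable piano that builds its keyboard from instanced white and black key meshes using a repeating key pattern.
; Interacting toggles cursor-hover tracing on Tick and triggers a camera blend, whose completion opens a menu.
; Clicks and keyboard input play MusicData sounds and write game time into per-instance custom data to animate keys.
; The menu shows the selected passcode hint, and its button starts a timer that plays that passcode's notes.
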(event `Key|AnyKey` :paused true
  (params (Key :type "Key Structure"))
  (bind _returnvalue (`KismetInputLibrary.Key_GetDisplayName` Key false))
  ;[1 1 1] Lazy input handler
  (:`Pressed`
    (switch `string` (`KismetTextLibrary.Conv_TextToString` _returnvalue)
      (:`1`
        _)
      (:`2`
        _)
      (:`3`
        _)
      (:`4`
        _)
      (:`5`
        _)
      (:`6`
        _)
      (:`7`
        _)
      (:`8`
        _)
      (:`9`
        _))
    (`self.PlayKey` (cast `/Game/Migrated/DataAssets/MusicKeys/E_MusicKeys` (`KismetMathLibrary.Conv_IntToByte` (`KismetStringLibrary.Conv_StringToInt` (`KismetTextLibrary.Conv_TextToString` _returnvalue)))))))

(event `self.ReceiveTick`
  (params (DeltaSeconds :type "Float (single-precision)"))
  (bind (_returnvalue _hitcomponent _hititem) (`self.CheckIfSameComponentUnderMouse`))
  ;[1 1 1] Tick (Starts Disabled) - Detects Components under mouse
  (if (not _returnvalue)
    (bind _asinstanced_static_mesh_component (cast `InstancedStaticMeshComponent` _hitcomponent))
    (set `self.ComponentUnderCursor` _asinstanced_static_mesh_component)
    (set `self.InstatncedStaticMeshIndex` _hititem)))

(event `/Game/Migrated/InteractionUpdated/I_InteractStartEnd.BeginInteract`
  (params (Player :type "/Game/ThirdPerson/Blueprints/BP_ThirdPersonCharacter Object Reference"))
  ;[1 1 1] Interaction
  (`self.SetActorTickEnabled` true)
  (`/Game/Migrated/Camera/AC_CameraBlend.Trigger` (`self.AC_CameraBlend`)))

(event `/Game/Migrated/InteractionUpdated/I_InteractStartEnd.EndInteract`
  (params (Player :type "/Game/ThirdPerson/Blueprints/BP_ThirdPersonCharacter Object Reference"))
  ;[1 1 1] Interaction
  (`self.SetActorTickEnabled` false)
  (set `self.InstatncedStaticMeshIndex` -1) ; Clear Animation Index under Cursor
  (`/Game/Migrated/Camera/AC_CameraBlend.Trigger` (`self.AC_CameraBlend`))
  ;;[1 1 1] close menu
  (`/Game/Migrated/AC_MenuController.Close` (`self.AC_MenuController`)))

(event `/Game/Interactable/I_Instrument.PlayKey`
  (params (Key :type "/Game/Migrated/DataAssets/MusicKeys/E_MusicKeys Enum" :default "NewEnumerator9"))
  ;[1 1 1] Play Key
  (`self.GetKeyComponent` (`KismetMathLibrary.Conv_ByteToInt` Key) 0 (`KismetSystemLibrary.GetGameTimeInSeconds`))
  (`self.PlaySound` (`self.MusicData`) Key))

(event `Key|LeftMouseButton`
  (params (Key :type "Key Structure"))
  ;[1 1 1] Handle Click events
  (:`Pressed`
    (`self.PlayAnimationKey` (`self.ComponentUnderCursor`) (`self.InstatncedStaticMeshIndex`))
    (bind _sound (`/Game/Migrated/DataAssets/MusicKeys/DA_MusicKeys.GetSoundByIndex` (`self.MusicData`) (`self.InstatncedStaticMeshIndex`)))
    (`GameplayStatics.PlaySound2D` _sound 1.0 1.0 0.0 null null)))

(event `self.AC_CameraBlend.OnComplete`
  ;[1 1 1] Camera Movement Event
  ;;[1 1 1] Open menu
  (`/Game/Migrated/AC_MenuController.Open` (`self.AC_MenuController`)))

(event `self.AC_UI_SubMenu.OnClick` :!enabledstate Disabled
  (params (ByteFlag :type Byte))
  (switch `|SwitchEnum` (cast `` ByteFlag)
    (:`NewEnumerator0`
      (`self.PlayHint`))
    (:`NewEnumerator1`
      (`self.HandleChangeHint`))))

(event `self.AC_UI_SubMenu.OnLoad` :!enabledstate Disabled
  (`self.HandleChangeHint`))

(event `self.AC_MenuController.OnLoad`
  (params (Widget :type "Widget Object Reference"))
  (bind _aswbp_test_piano (cast `/Game/UI/Interactable/Piano/WBP_Test_Piano` Widget))
  (set `self.InfoText` (`/Game/UI/Interactable/Piano/WBP_Test_Piano.TextBlock` _aswbp_test_piano))
  (add `Button.OnClicked` (`/Game/UI/Interactable/Piano/WBP_Test_Piano.Button_0` _aswbp_test_piano) (delegate `CustomEvent`))
  (`self.HandleChangeHint`))

(event `CustomEvent`
  (bind _returnvalue (`KismetSystemLibrary.K2_SetTimerDelegate` (delegate `Tick`) 0.4))
  (set `self.HintTimerHandler` _returnvalue))

(event `Tick`
  (`self.PlayKey` (`/Game/Migrated/DataAssets/MusicKeys/DA_Passcode.Get` (`|GetArrayItem` (`self.PassCodeList`) (`self.PassCodeListIndex`)) (`self.PassCodeListIndex`)))
  (bind _result (`/Engine/EditorBlueprintResources/StandardMacros.IncrementInt` (`self.Index`))
    (:`  `
      (if (>= _result (`KismetArrayLibrary.Array_Length` (`/Game/Migrated/DataAssets/MusicKeys/DA_Passcode.Passcode` (`|GetArrayItem` (`self.PassCodeList`) (`self.PassCodeListIndex`)))))
        (`KismetSystemLibrary.K2_ClearAndInvalidateTimerHandle` (`self.HintTimerHandler`))
        (set `self.Index` 0)))))

(fn `CheckIfSameComponentUnderMouse`
  (returns (ReturnValue :type Boolean) (HitComponent :type "PrimitiveComponent Object Reference") (HitItem :type Integer))
  (bind (_hitcomponent _hititem) (`self.GetCursorHitIndex`))
  (return (and (== _hititem (`self.InstatncedStaticMeshIndex`)) (== _hitcomponent (`self.ComponentUnderCursor`))) _hitcomponent _hititem))

(fn `GetCursorHitIndex`
  (returns (HitComponent :type "PrimitiveComponent Object Reference") (HitItem :type Integer))
  (bind (_bblockinghit _binitialoverlap _time _distance _location _impactpoint _normal _impactnormal _physmat _hitactor _hitcomponent _hitbonename _bonename _hititem) (`GameplayStatics.BreakHitResult` (`PlayerController.GetHitResultUnderCursorByChannel` (`GameplayStatics.GetPlayerController` 0) "TraceTypeQuery1" false)))
  (return _hitcomponent _hititem))

(fn `GetKeyComponent`
  (params (Index :type Integer) (CustomDataIndex :type Integer) (CustomDataValue :type "Float (single-precision)"))
  (locals (NewLocalVar :type Integer))
  (set `local.NewLocalVar` (`BlueprintMapLibrary.Map_Find` (`self.KeyMap`) Index))
  (if (`|GetArrayItem` (`self.KeySettingMap`) (mod Index (`KismetArrayLibrary.Array_Length` (`self.KeySettingMap`))))
    (`InstancedStaticMeshComponent.SetCustomDataValue` (`self.BlackKeys`) (`local.NewLocalVar`) CustomDataIndex CustomDataValue true)
    (else
      (`InstancedStaticMeshComponent.SetCustomDataValue` (`self.WhiteKeys`) (`local.NewLocalVar`) CustomDataIndex CustomDataValue true))))

(fn `HandleChangeHint`
  (set `self.PassCodeListIndex` (mod (+ (`self.PassCodeListIndex`) 1) (`KismetArrayLibrary.Array_Length` (`self.PassCodeList`))))
  (set `TextBlock.Text` (`KismetTextLibrary.Conv_StringToText` (`KismetSystemLibrary.GetDisplayName` (`|GetArrayItem` (`self.PassCodeList`) (`self.PassCodeListIndex`)))) (`self.InfoText`))
  (return))

(fn `PlayAnimationKey`
  (params (PianoKeyInstanceSet :type "InstancedStaticMeshComponent Object Reference") (InstanceIndex :type Integer))
  (`InstancedStaticMeshComponent.SetCustomDataValue` PianoKeyInstanceSet InstanceIndex 0 (`KismetSystemLibrary.GetGameTimeInSeconds`) true)
  (return))

(fn `PlayHint`
  (return))

(fn `PlaySound`
  (params (self2 :type "/Game/Migrated/DataAssets/MusicKeys/DA_MusicKeys Object Reference") (Key :type "Byte (by ref)"))
  (bind _value (`/Game/Migrated/DataAssets/MusicKeys/DA_MusicKeys.GetSound` self2 (cast `/Game/Migrated/DataAssets/MusicKeys/E_MusicKeys` Key)))
  (`GameplayStatics.PlaySound2D` _value 1.0 1.0 0.0 null null))

(fn `UserConstructionScript`
  (locals (LocalIndex :type Integer) (LocalOffset :type "Vector Structure" :default (0.0 0.0 0.0)) (LocalBlackXOffset :type "Float (double-precision)"))
  (`parent.UserConstructionScript`)
  (set `local.LocalBlackXOffset` (/ (`self.WhiteKeyXOffset`) 2.0))
  (for _index (range (`self.Start`) (+ (+ (`self.Start`) (`self.Count`) -1) 1))
    (bind _output_get (set `local.LocalIndex` _index))
    (if (`|GetArrayItem` (`self.KeySettingMap`) (mod _output_get 12))
      (bind _returnvalue (`InstancedStaticMeshComponent.AddInstance` (`self.BlackKeys`) (`KismetMathLibrary.MakeTransform` (+ (`local.LocalOffset`) (`KismetMathLibrary.MakeVector` (`local.LocalBlackXOffset`) 0.0 (`self.BlackKeyZOffset`)))) false))
      (`BlueprintMapLibrary.Map_Add` (`self.KeyMap`) (`local.LocalIndex`) _returnvalue)
      (else
        (bind _output_get_2 (set `local.LocalOffset` (+ (`local.LocalOffset`) (`KismetMathLibrary.MakeVector` (`self.WhiteKeyXOffset`)))))
        (bind _returnvalue_2 (`InstancedStaticMeshComponent.AddInstance` (`self.WhiteKeys`) (`KismetMathLibrary.MakeTransform` _output_get_2) false))
        (`BlueprintMapLibrary.Map_Add` (`self.KeyMap`) (`local.LocalIndex`) _returnvalue_2)))))